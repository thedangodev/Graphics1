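; Test player Blueprint for the FPS folder that spawns an actor at an enemy spawn point and tracks its own death.
; On BeginPlay it spawns the actor at EnemySpawnPoint's transform, passing itself as PlayerRef.
; Tick polls Health and, the first time it drops below zero, sets IsDead and prints a death message.
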(event `self.ReceiveBeginPlay`
  (`|SpawnActorFromClass` "/Game/FPS/BP_TestEnemy.BP_TestEnemy_C" (`self.GetTransform` (`self.EnemySpawnPoint`)) "Undefined" "MultiplyWithRoot" null self null))

(event `self.ReceiveTick`
  (params (DeltaSeconds :type "Float (single-precision)"))
  (if (and (== (`self.IsDead`) false) (< (`self.Health`) 0.0))
    (set `self.IsDead` true)
    (`KismetSystemLibrary.PrintString` "I'm dead now!")))

(fn `UserConstructionScript`)